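; BP_HistoryMap is a level-select map actor that reacts when the map pawn enters its collision box.
; On overlap it casts to BP_MapPawn, stores a reference and switches on its Statename value.
; The Va case moves the pawn to this actor's location, while Ny, Ga and the default case only print debug strings.
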(event `self.BoxCollision.OnComponentBeginOverlap`
  (params (OverlappedComponent :type "PrimitiveComponent Object Reference") (OtherActor :type "Actor Object Reference") (OtherComp :type "PrimitiveComponent Object Reference") (OtherBodyIndex :type Integer) (bFromSweep :type Boolean) (SweepResult :type "HitResult Structure (by ref)"))
  (bind (_returnvalue_x _returnvalue_y _returnvalue_z) (`KismetMathLibrary.BreakVector` (`self.K2_GetActorLocation`)))
  (bind _asbp_map_pawn (cast `/Game/LevelSelect/BP_MapPawn` OtherActor))
  (set `self.MapPawnRef` _asbp_map_pawn)
  (switch `name` (`self.Statename`)
    (:`Default`
      (`KismetSystemLibrary.PrintString` "default"))
    (:`va`
      (`KismetSystemLibrary.PrintString` "Va")
      (`self.K2_SetActorLocation` (`self.MapPawnRef`) (`KismetMathLibrary.MakeVector` _returnvalue_x _returnvalue_y _returnvalue_z) false false)
      (`KismetSystemLibrary.PrintString` "Hello"))
    (:`ny`
      (`KismetSystemLibrary.PrintString` "Ny"))
    (:`ga`
      (`KismetSystemLibrary.PrintString` "Ga"))))

(fn `UserConstructionScript`)