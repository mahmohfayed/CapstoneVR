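; BP_MasterMenu is a VR menu actor that drives two-handed laser pointer interaction with widgets.
; It finds the player pawn's widget interaction and aim motion controller components, retrying on a timer until all are valid, then snaps each interactor to its controller.
; Trigger inputs become left-mouse pointer clicks.
; Tick moves Niagara lasers and cursors to the hit points, showing each only while its hand points at a focusable widget.
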(event `InputAction|TriggerLeft`
  (params (Key :type "Key Structure"))
  (bind _widgetinteractionrefl (`self.WidgetInteractionRefL`))
  (:`Pressed`
    (`KismetSystemLibrary.PrintString` "Pressed")
    (`WidgetInteractionComponent.PressPointerKey` _widgetinteractionrefl "LeftMouseButton"))
  (:`Released`
    (`KismetSystemLibrary.PrintString` "Release")
    (`WidgetInteractionComponent.ReleasePointerKey` _widgetinteractionrefl "LeftMouseButton")))

(event `InputAction|TriggerRight`
  (params (Key :type "Key Structure"))
  (bind _widgetinteractionrefr (`self.WidgetInteractionRefR`))
  (:`Pressed`
    (`KismetSystemLibrary.PrintString` "Pressed")
    (`WidgetInteractionComponent.PressPointerKey` _widgetinteractionrefr "LeftMouseButton"))
  (:`Released`
    (`KismetSystemLibrary.PrintString` "Release")
    (`WidgetInteractionComponent.ReleasePointerKey` _widgetinteractionrefr "LeftMouseButton")))

(event `self.ReceiveBeginPlay`
  ;[1 1 1] Initialize Left and Right motion controller, Enable Input
  (`self.EnableInput` (`GameplayStatics.GetPlayerController` 0))
  (`self.SetWidgetInteractionReferences`)
  (`self.SetMotionControllerReference`)
  ;[1 1 1] Try and get all Motion controller components to initialize
  (if (not (and (`KismetSystemLibrary.IsValid` (`self.WidgetInteractionRefL`)) (`KismetSystemLibrary.IsValid` (`self.WidgetInteractionRefR`)) (`KismetSystemLibrary.IsValid` (`self.MotionControllerAimRefL`)) (`KismetSystemLibrary.IsValid` (`self.MotionControllerAimRefR`))))
    (bind _returnvalue (`KismetSystemLibrary.K2_SetTimerDelegate` (delegate `TryToAddMCRef`) 1.0 true))
    (set `self.AddMCRefTimerHandle` _returnvalue)))

(event `TryToAddMCRef`
  ;[1 1 1] Try and get all Motion controller components to initialize
  (`self.SetWidgetInteractionReferences`)
  (`self.SetMotionControllerReference`)
  (if (and (`KismetSystemLibrary.IsValid` (`self.WidgetInteractionRefL`)) (`KismetSystemLibrary.IsValid` (`self.WidgetInteractionRefR`)) (`KismetSystemLibrary.IsValid` (`self.MotionControllerAimRefL`)) (`KismetSystemLibrary.IsValid` (`self.MotionControllerAimRefR`)))
    (`KismetSystemLibrary.K2_ClearAndInvalidateTimerHandle` (`self.AddMCRefTimerHandle`))))

(event `self.ReceiveTick`
  (params (DeltaSeconds :type "Float (single-precision)"))
  (if (or (`KismetSystemLibrary.IsValid` (`self.MotionControllerAimRefL`)) (`KismetSystemLibrary.IsValid` (`self.MotionControllerAimRefR`)))
    (if (or (`KismetSystemLibrary.IsValid` (`self.WidgetInteractionRefL`)) (`KismetSystemLibrary.IsValid` (`self.WidgetInteractionRefR`)))
      (`|ExecutionSequence`
        (:`then_0`
          (`|ExecutionSequence`
            (:`then_0`
              ;[1 1 1] Show MenuLaser
              (`/Engine/EditorBlueprintResources/StandardMacros.DoOnce` false
                (:`Completed`
                  (`SceneComponent.K2_AttachToComponent` (`self.WidgetInteractionRefL`) (`self.MotionControllerAimRefL`) "None" "SnapToTarget" "SnapToTarget" "KeepWorld" true) ; Attach WIC to MotionController
                  (`SceneComponent.K2_AttachToComponent` (`self.WidgetInteractionRefR`) (`self.MotionControllerAimRefR`) "None" "SnapToTarget" "SnapToTarget" "KeepWorld" true) ; Attach WIC to MotionController
                )))
            (:`then_1`
              ;[1 1 1] Update MenuLaser endpoint, Update Cursor location
              (`self.UpdateMenuLaser` (`self.CursorR`) (`self.MenuLaserR`) (`self.WidgetInteractionRefR`))
              (`self.UpdateMenuLaser` (`self.CursorL`) (`self.MenuLaserL`) (`self.WidgetInteractionRefL`)))))
        (:`then_1`
          (`/Engine/EditorBlueprintResources/StandardMacros.DoOnce` false :!label _label
            (:`Completed`
              (`self.SetHidden` (`WidgetInteractionComponent.IsOverFocusableWidget` (`self.WidgetInteractionRefL`)) (`WidgetInteractionComponent.IsOverFocusableWidget` (`self.WidgetInteractionRefR`))))))
        (:`then_2`
          (if (or (!= (`WidgetInteractionComponent.IsOverFocusableWidget` (`self.WidgetInteractionRefL`)) (`self.bLastFocus_L`)) (!= (`WidgetInteractionComponent.IsOverFocusableWidget` (`self.WidgetInteractionRefR`)) (`self.bLastFocus_R`)))
            (goto _label :!via `Reset`)))))))

(fn `GetWidgetInteractionComponent`
  (params (bRightWIC :type Boolean))
  (returns (ReturnValue :type "WidgetInteractionComponent Object Reference"))
  (return (select `bool` bRightWIC :`false` (`self.WidgetInteractionRefL`) :`true` (`self.WidgetInteractionRefR`))))

(fn `SetHidden`
  (params (bIsFocusedL :type Boolean) (bIsFocusedR :type Boolean))
  (bind _bisfocusedl (`local.bIsFocusedL`))
  (bind _bisfocusedr (`local.bIsFocusedR`))
  (`|ExecutionSequence`
    (:`then_0`
      (`SceneComponent.SetHiddenInGame` (`self.MenuLaserL`) (not _bisfocusedl) false)
      (`SceneComponent.SetHiddenInGame` (`self.CursorL`) (not _bisfocusedl) false)
      (set `self.bLastFocus_L` _bisfocusedl))
    (:`then_1`
      (`SceneComponent.SetHiddenInGame` (`self.CursorR`) (not _bisfocusedr) false)
      (`SceneComponent.SetHiddenInGame` (`self.MenuLaserR`) (not _bisfocusedr) false)
      (set `self.bLastFocus_R` _bisfocusedr))))

(fn `SetMotionControllerReference`
  (locals (LocalMotionControllers :type "Array of MotionControllerComponent Object Reference"))
  (bind _returnvalue (`self.K2_GetComponentsByClass` (`GameplayStatics.GetPlayerPawn` 0) "/Script/HeadMountedDisplay.MotionControllerComponent"))
  (if (> (`KismetArrayLibrary.Array_Length` _returnvalue) 0)
    (bind _output_get (set `local.LocalMotionControllers` _returnvalue))
    (for _array_element _output_get
      (switch `name` (`MotionControllerComponent.MotionSource` _array_element)
        (:`LeftAim`
          (set `self.MotionControllerAimRefL` _array_element)
          (`KismetSystemLibrary.PrintString` "LeftHand MotionController Set" true true (struct :`R` 1.0 :`G` 0.90171 :`A` 1.0) 10.0))
        (:`RightAim`
          (set `self.MotionControllerAimRefR` _array_element)
          (`KismetSystemLibrary.PrintString` "RightHand MotionController Set" true true (struct :`R` 1.0 :`G` 0.90171 :`A` 1.0) 10.0))))
    (else
      (`KismetSystemLibrary.PrintString` "Warning: No WidgetInteractionComponent was found. Menu interaction will FAIL"))))

(fn `SetWidgetInteractionReferences`
  (locals (LocalWidgetInteractionComponents :type "Array of WidgetInteractionComponent Object Reference"))
  (bind _returnvalue (`self.K2_GetComponentsByClass` (`GameplayStatics.GetPlayerPawn` 0) "/Script/UMG.WidgetInteractionComponent"))
  (if (> (`KismetArrayLibrary.Array_Length` _returnvalue) 0)
    (bind _output_get (set `local.LocalWidgetInteractionComponents` _returnvalue))
    (for _array_element _output_get
      (if (== (`WidgetInteractionComponent.PointerIndex` _array_element) 0)
        (set `self.WidgetInteractionRefL` _array_element)
        (else
          (set `self.WidgetInteractionRefR` _array_element))))
    (else
      (`KismetSystemLibrary.PrintString` "Warning: No WidgetInteractionComponent was found. Menu interaction will FAIL"))))

(fn `UpdateMenuLaser`
  (params (Cursor :type "SceneComponent Object Reference") (MenuLaser :type "NiagaraComponent Object Reference") (WidgetInteractComp :type "WidgetInteractionComponent Object Reference"))
  (bind (_returnvalue_bblockinghit _returnvalue_binitialoverlap _returnvalue_time _returnvalue_distance _returnvalue_location _returnvalue_impactpoint) (`GameplayStatics.BreakHitResult` (`WidgetInteractionComponent.GetLastHitResult` WidgetInteractComp)))
  (`SceneComponent.K2_SetWorldLocation` Cursor _returnvalue_impactpoint false false)
  (`NiagaraDataInterfaceArrayFunctionLibrary.SetNiagaraArrayVectorValue` (`local.MenuLaser`) "User.PointArray" 0 (`SceneComponent.K2_GetComponentLocation` (`local.WidgetInteractComp`))) ; MenuLaser start location
  (`NiagaraDataInterfaceArrayFunctionLibrary.SetNiagaraArrayVectorValue` (`local.MenuLaser`) "User.PointArray" 1 _returnvalue_impactpoint) ; MenuLaser end location
)

(fn `UserConstructionScript`)