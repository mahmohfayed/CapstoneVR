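; BP_MPTestPawn is a simple pawn in the LevelSelect folder, apparently for multiplayer testing.
; On BeginPlay it switches the first player controller to UI-only input without mouse lock and shows the cursor.
; Axis events add movement along the camera's forward and right vectors and feed look input into controller pitch and yaw.
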(event `self.ReceiveBeginPlay`
  (bind _returnvalue (`GameplayStatics.GetPlayerController` 0))
  (`WidgetBlueprintLibrary.SetInputMode_UIOnlyEx` _returnvalue null)
  (set `PlayerController.bShowMouseCursor` true _returnvalue))

(event `InputAxis|3PF`
  (params (AxisValue :type "Float (single-precision)"))
  (`self.AddMovementInput` (`SceneComponent.GetForwardVector` (`self.Camera`)) AxisValue))

(event `InputAxis|3PR`
  (params (AxisValue :type "Float (single-precision)"))
  (`self.AddMovementInput` (`SceneComponent.GetRightVector` (`self.Camera`)) AxisValue))

(event `InputAxis|3PLookUp/Down`
  (params (AxisValue :type "Float (single-precision)"))
  (`self.AddControllerPitchInput` AxisValue))

(event `InputAxis|3PLookRight/Left`
  (params (AxisValue :type "Float (single-precision)"))
  (`self.AddControllerYawInput` AxisValue))

(fn `UserConstructionScript`)