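; VR multiple-choice question station with three grabbable answers that awards a trophy for a correct first try.
; CreateBases fills question and answer widgets and finds the BP_TrophyCountBoard; everything stays hidden until a VRPawn enters the standing ring.
; Holding an answer for five seconds fires its Glow event via a timer, cancelled on drop.
; Glow recolors the gem, adding particles and a trophy if no wrong answer came first; only answer 1 plays sounds.
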(event `self.ReceiveBeginPlay`
  (`SceneComponent.SetVisibility` (`self.Root`) false true)
  (`SceneComponent.SetVisibility` (`self.StandingRing`) true false))

(event `CreateBases`
  (params (Question_text :type Text) (answer_1 :type Text) (answer_2 :type Text) (answer_3 :type Text) (correct_answer :type Integer))
  ;[1 1 1] Prepare Trophy Base
  (`|ExecutionSequence`
    (:`then_0`
      (bind _returnvalue (`|CreateWidget` "/Game/Language/Blueprints/Trophy/WBP_Question.WBP_Question_C" null Question_text))
      (`WidgetComponent.SetWidget` (`self.Question`) _returnvalue)
      (bind _returnvalue_2 (`|CreateWidget` "/Game/Language/Blueprints/Trophy/WBP_Question.WBP_Question_C" null answer_1))
      (`WidgetComponent.SetWidget` (`self.Answer1`) _returnvalue_2)
      (bind _returnvalue_3 (`|CreateWidget` "/Game/Language/Blueprints/Trophy/WBP_Question.WBP_Question_C" null answer_2))
      (`WidgetComponent.SetWidget` (`self.Answer2`) _returnvalue_3)
      (bind _returnvalue_4 (`|CreateWidget` "/Game/Language/Blueprints/Trophy/WBP_Question.WBP_Question_C" null answer_3))
      (`WidgetComponent.SetWidget` (`self.Answer3`) _returnvalue_4)
      (set `self.correct_answer` correct_answer)
      (bind _returnvalue_5 (`GameplayStatics.GetActorOfClass` "/Game/Language/Blueprints/Points/BP_TrophyCountBoard.BP_TrophyCountBoard_C"))
      (set `self.Point Board` _returnvalue_5))
    (:`then_1`
      (`SceneComponent.SetVisibility` (`self.Answer1`) false false)
      (`SceneComponent.SetVisibility` (`self.Answer2`) false false)
      (`SceneComponent.SetVisibility` (`self.Answer3`) false false)
      (`SceneComponent.SetVisibility` (`self.Question`) false false))))

(event `self.StandingRing.OnComponentBeginOverlap`
  (params (OverlappedComponent :type "PrimitiveComponent Object Reference") (OtherActor :type "Actor Object Reference") (OtherComp :type "PrimitiveComponent Object Reference") (OtherBodyIndex :type Integer) (bFromSweep :type Boolean) (SweepResult :type "HitResult Structure (by ref)"))
  ;[1 0.9704 0.1156] Set Visible when Approaching
  (cast `/Game/VRTemplate/Blueprints/VRPawn` OtherActor)
  (`/Engine/EditorBlueprintResources/StandardMacros.DoOnce` false
    (:`Completed`
      (`SceneComponent.SetVisibility` (`self.Root`) true true)
      (`SceneComponent.SetVisibility` (`self.StandingRing`) false false))))

(event `self.GrabComponent2.OnDropped`
  ;[1 0.4902 0.2353] Answer Choice 2
  (`KismetSystemLibrary.K2_ClearAndInvalidateTimerHandle` (stale `self.GrabComponent2.OnGrabbed` _returnvalue)))

(event `self.GrabComponent3.OnDropped`
  ;[1 0.4902 0.2353] Answer Choice 3
  (`KismetSystemLibrary.K2_ClearAndInvalidateTimerHandle` (stale `self.GrabComponent3.OnGrabbed` _returnvalue)))

(event `self.GrabComponent1.OnDropped`
  ;[1 0.4902 0.2353] Answer Choice 1
  (`KismetSystemLibrary.K2_ClearAndInvalidateTimerHandle` (stale `self.GrabComponent1.OnGrabbed` _returnvalue)))

(event `self.GrabComponent2.OnGrabbed`
  ;[1 0.4902 0.2353] Answer Choice 2
  (bind _returnvalue (`KismetSystemLibrary.K2_SetTimerDelegate` (delegate `Glow2`) 5.0)))

(event `self.GrabComponent3.OnGrabbed`
  ;[1 0.4902 0.2353] Answer Choice 3
  (bind _returnvalue (`KismetSystemLibrary.K2_SetTimerDelegate` (delegate `Glow3`) 5.0)))

(event `self.GrabComponent1.OnGrabbed`
  ;[1 0.4902 0.2353] Answer Choice 1
  (bind _returnvalue (`KismetSystemLibrary.K2_SetTimerDelegate` (delegate `Glow1`) 5.0)))

(event `Glow2`
  ;[1 0.4902 0.2353] Answer Choice 2
  (if (== (`self.correct_answer`) 2)
    (`PrimitiveComponent.SetMaterial` (`self.Gem2`) 0 "/Engine/MapTemplates/Materials/BasicAsset03.BasicAsset03")
    (if (`self.first_time`)
      (`ActorComponent.Activate` (`self.Niagara2`) false)
      (`/Engine/EditorBlueprintResources/StandardMacros.DoOnce` false
        (:`Completed`
          (`/Game/Language/Blueprints/Points/BP_TrophyCountBoard.Add_Trophy` (`self.Point Board`)))))
    (else
      (`PrimitiveComponent.SetMaterial` (`self.Gem2`) 0 "/Engine/MapTemplates/Materials/BasicAsset01.BasicAsset01")
      (set `self.first_time` false))))

(event `Glow3`
  ;[1 0.4902 0.2353] Answer Choice 3
  (if (== (`self.correct_answer`) 3)
    (`PrimitiveComponent.SetMaterial` (`self.Gem3`) 0 "/Engine/MapTemplates/Materials/BasicAsset03.BasicAsset03")
    (if (`self.first_time`)
      (`ActorComponent.Activate` (`self.Niagara3`) false)
      (`/Engine/EditorBlueprintResources/StandardMacros.DoOnce` false
        (:`Completed`
          (`/Game/Language/Blueprints/Points/BP_TrophyCountBoard.Add_Trophy` (`self.Point Board`)))))
    (else
      (`PrimitiveComponent.SetMaterial` (`self.Gem3`) 0 "/Engine/MapTemplates/Materials/BasicAsset01.BasicAsset01")
      (set `self.first_time` false))))

(event `Glow1`
  ;[1 0.4902 0.2353] Answer Choice 1
  (if (== (`self.correct_answer`) 1)
    (`PrimitiveComponent.SetMaterial` (`self.Gem1`) 0 "/Engine/MapTemplates/Materials/BasicAsset03.BasicAsset03")
    (`GameplayStatics.PlaySound2D` "/Game/Language/Sounds/correct_answer_tone.correct_answer_tone" 1.0 1.0 0.0 null null)
    (if (`self.first_time`)
      (`ActorComponent.Activate` (`self.Niagara1`) false)
      (`/Engine/EditorBlueprintResources/StandardMacros.DoOnce` false
        (:`Completed`
          (`/Game/Language/Blueprints/Points/BP_TrophyCountBoard.Add_Trophy` (`self.Point Board`)))))
    (else
      (`PrimitiveComponent.SetMaterial` (`self.Gem1`) 0 "/Engine/MapTemplates/Materials/BasicAsset01.BasicAsset01")
      (`GameplayStatics.PlaySound2D` "/Game/Language/Sounds/wrong-buzzer.wrong-buzzer" 1.0 1.0 0.0 null null)
      (set `self.first_time` false))))

(fn `UserConstructionScript`)