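; Puzzle lever that triggers a slot check on a referenced translate display when pulled.
; Each tick, the cube's Y offset from an arrow drives the handle's pitch within a clamped range, then the cube snaps back to the arrow.
; Overlap between handle and activation collisions fires the check through a DoOnce, then after a delay restores the cube's starting transform and resets the display's check.
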(event `self.ReceiveTick`
  (params (DeltaSeconds :type "Float (single-precision)"))
  (bind _lever (`self.Lever`))
  (bind _translatedisplayref (`self.TranslateDisplayRef`))
  (bind (_returnvalue_roll _returnvalue_pitch _returnvalue_yaw) (`KismetMathLibrary.BreakRotator` (`SceneComponent.K2_GetComponentRotation` _lever)))
  (bind (_returnvalue_location _returnvalue_rotation) (`KismetMathLibrary.BreakTransform` (`SceneComponent.K2_GetComponentToWorld` (`self.Arrow`))))
  (bind (_returnvalue_x _returnvalue_y) (`KismetMathLibrary.BreakVector` (- (`SceneComponent.K2_GetComponentLocation` (`self.Arrow`)) (`SceneComponent.K2_GetComponentLocation` (`self.Cube`)))))
  (`|ExecutionSequence`
    (:`then_0`
      ;[1 1 1] When the cube moves, move the handle
      (`SceneComponent.K2_SetWorldRotation` _lever (`KismetMathLibrary.MakeRotator` _returnvalue_roll (`KismetMathLibrary.FClamp` (+ _returnvalue_pitch _returnvalue_y) -30.0 30.0) _returnvalue_yaw) false false)
      (`SceneComponent.K2_SetWorldLocationAndRotation` (`self.Cube`) _returnvalue_location _returnvalue_rotation false false))
    (:`then_1`
      (if (`PrimitiveComponent.IsOverlappingComponent` (`self.HandleCollision`) (`self.ActivatedCollision`))
        ;[1 1 1] Check the slots
        (`/Engine/EditorBlueprintResources/StandardMacros.DoOnce` false :!label _label
          (:`Completed`
            (`/Game/Language/Blueprints/Puzzles/Sentences/BP_TranslateDisplay.CheckAllSlots` _translatedisplayref)
            (`KismetSystemLibrary.Delay` 2.0)
            (`SceneComponent.K2_SetWorldTransform` (`self.Cube`) (`self.OriginalTransform`) false false)
            (`/Game/Language/Blueprints/Puzzles/Sentences/BP_TranslateDisplay.ResetSlotCheck` _translatedisplayref)))
        (else
          (goto _label :!via `Reset`))))))

(event `self.ReceiveBeginPlay`
  ;[1 1 1] Set the original location of cube (and lever handle)
  (set `self.OriginalTransform` (`SceneComponent.K2_GetComponentToWorld` (`self.Cube`))))

(fn `UserConstructionScript`)