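; BP_PuzzleSlot is a slot on a VR puzzle board that accepts one BP_PuzzlePiece at a time.
; A piece entering the box collision is released from the player's grab and snapped to the box transform if the slot is empty.
; A matching piece marks the slot correct and asks the board to check all slots, while removing it resets the slot.
; PuzzleCompleted turns the cube emissive green.
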(event `self.ReceiveBeginPlay`
  (bind _asvrpawn (cast `/Game/VRTemplate/Blueprints/VRPawn` (`GameplayStatics.GetPlayerPawn` 0)))
  (set `self.As VRPawn` _asvrpawn))

(event `self.Box Collision.OnComponentBeginOverlap`
  (params (OverlappedComponent :type "PrimitiveComponent Object Reference") (OtherActor :type "Actor Object Reference") (OtherComp :type "PrimitiveComponent Object Reference") (OtherBodyIndex :type Integer) (bFromSweep :type Boolean) (SweepResult :type "HitResult Structure (by ref)"))
  (bind (_returnvalue_location _returnvalue_rotation) (`KismetMathLibrary.BreakTransform` (`SceneComponent.K2_GetComponentToWorld` (`self.Box Collision`))))
  (bind _asbp_puzzle_piece (cast `/Game/Language/Blueprints/Puzzles/Puzzle/BP_PuzzlePiece` OtherActor))
  (`/Engine/EditorBlueprintResources/StandardMacros.IsValid` (`self.CurrentPiece`)
    (:`Is Not Valid`
      (bind _output_get (set `self.CurrentPiece` _asbp_puzzle_piece))
      (`/Game/VRTemplate/Blueprints/GrabComponent.TryRelease` (`/Game/Language/Blueprints/Puzzles/Puzzle/BP_PuzzlePiece.GrabComponent` _output_get))
      (`self.K2_SetActorLocationAndRotation` _asbp_puzzle_piece _returnvalue_location _returnvalue_rotation false false)
      (if (== (`/Game/Language/Blueprints/Puzzles/Puzzle/BP_PuzzlePiece.Slot` _output_get) (`self.Piece`))
        (set `self.Correct` true)
        (`/Game/Language/Blueprints/Puzzles/Puzzle/BP_PuzzleBoard.CheckAllCorrect` (`self.PuzzleBoardRef`))))))

(event `self.Box Collision.OnComponentEndOverlap`
  (params (OverlappedComponent :type "PrimitiveComponent Object Reference") (OtherActor :type "Actor Object Reference") (OtherComp :type "PrimitiveComponent Object Reference") (OtherBodyIndex :type Integer))
  (bind _asbp_puzzle_piece (cast `/Game/Language/Blueprints/Puzzles/Puzzle/BP_PuzzlePiece` OtherActor))
  (if (== _asbp_puzzle_piece (`self.CurrentPiece`))
    (set `self.CurrentPiece` null)
    (set `self.Correct` false)))

(event `PuzzleCompleted`
  (`PrimitiveComponent.SetMaterial` (`self.Cube`) 0 "/Game/Language/Materials/Emissives/M_Emissive_Green.M_Emissive_Green"))

(fn `UserConstructionScript`)