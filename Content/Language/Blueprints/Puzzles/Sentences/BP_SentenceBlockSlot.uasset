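; BP_SentenceBlockSlot is a slot in a sentence puzzle that reports whether the word block placed in it is the correct one.
; ReturnBlockCorrect takes the first BP_SentenceBlock overlapping BoxCollision, stores it as CenteredBlock and compares its BlockText to WordToMatch.
; The check runs only when called, as the overlap events are empty.
; Logic for snapping the block into place and tracking BlockCorrect is left disconnected.
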(event `self.Box Collision.OnComponentBeginOverlap`
  (params (OverlappedComponent :type "PrimitiveComponent Object Reference") (OtherActor :type "Actor Object Reference") (OtherComp :type "PrimitiveComponent Object Reference") (OtherBodyIndex :type Integer) (bFromSweep :type Boolean) (SweepResult :type "HitResult Structure (by ref)")))

(event `self.Box Collision.OnComponentEndOverlap`
  (params (OverlappedComponent :type "PrimitiveComponent Object Reference") (OtherActor :type "Actor Object Reference") (OtherComp :type "PrimitiveComponent Object Reference") (OtherBodyIndex :type Integer)))

(fn `Return Block Correct`
  (returns (BCorrect :type Boolean))
  ;[0.6827 0.3853 1] Center the Block
  (bind _asbp_sentence_block (cast `/Game/Language/Blueprints/Puzzles/Sentences/BP_SentenceBlock` (`|GetArrayItem` (`PrimitiveComponent.GetOverlappingActors` (`self.Box Collision`) "/Game/Language/Blueprints/Puzzles/Sentences/BP_SentenceBlock.BP_SentenceBlock_C"))))
  ;[0.8574 0.5546 1] Check if Block Word Matches
  (bind _output_get (set `self.CenteredBlock` _asbp_sentence_block))
  (return (== (`/Game/Language/Blueprints/Vocab/BP_VocabularyBlock.Block Text` _output_get) (`self.WordToMatch`))))

(fn `UserConstructionScript`
  (`parent.UserConstructionScript`))