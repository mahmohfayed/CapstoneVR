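; BP_VocabularyBlock is a word block for a vocabulary game that shows its text through six widget components and expires after a set lifespan.
; ChangeCorrect and ChangeWrong swap the cube's material to green or red neon.
; Once CreateExtraHits binds the hit event, the first hit on a BP_VocabTarget turns the block red and subtracts points.
; The construction script collects neon siding pieces, but the loops that would recolor them are unconnected.
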(event `CreateExtraHits`
  (params (PointsBoard :type "/Game/Language/Blueprints/Points/BP_VocabPointsBoard Object Reference"))
  ;[1 0.2486 0.7981] Hit Event - Subtract
  (add `self.OnActorHit` (delegate `ExtraBlockHits`)))

(event `ExtraBlockHits` :!signature `self.OnActorHit`
  (params (SelfActor :type "Actor Object Reference") (OtherActor :type "Actor Object Reference") (NormalImpulse :type "Vector Structure") (Hit :type "HitResult Structure (by ref)"))
  ;[1 0.2486 0.7981] Hit Event - Subtract
  (cast `/Game/Language/Blueprints/Vocab/BP_VocabTarget` OtherActor)
  (`/Engine/EditorBlueprintResources/StandardMacros.DoOnce` false
    (:`Completed`
      (`self.ChangeWrong`)
      (`/Game/Language/Blueprints/Points/BP_VocabPointsBoard.SubtractPoints` (stale `CreateExtraHits` PointsBoard))
      (`KismetSystemLibrary.Delay` 1.5))))

(event `self.ReceiveBeginPlay`
  ;[0.461 0.5606 1] Create Word Widgets (Surface)
  (bind _returnvalue (`|CreateWidget` "/Game/Language/Blueprints/Vocab/WBP_VocabText.WBP_VocabText_C" null (`self.Block Text`)))
  (`WidgetComponent.SetWidget` (`self.Word1`) _returnvalue)
  (`WidgetComponent.SetWidget` (`self.Word2`) _returnvalue)
  (`WidgetComponent.SetWidget` (`self.Word3`) _returnvalue)
  (`WidgetComponent.SetWidget` (`self.Word4`) _returnvalue)
  (`WidgetComponent.SetWidget` (`self.Word5`) _returnvalue)
  (`WidgetComponent.SetWidget` (`self.Word6`) _returnvalue)
  (`self.SetLifeSpan` (`self.Lifespan`)))

(event `ChangeCorrect`
  ;[0.02494 1 0.1983] Correct Neon
  (`PrimitiveComponent.SetMaterial` (`self.Cube`) 0 "/Game/Language/Materials/MI_tron_green.MI_tron_green"))

(event `ChangeWrong`
  ;[1 0.09279 0.1326] Wrong Neon
  (`PrimitiveComponent.SetMaterial` (`self.Cube`) 0 "/Game/Language/Materials/MI_tron_red.MI_tron_red"))

(fn `UserConstructionScript`
  (for _array_element (`|MakeArray` null null null null null null null null :!type "ChildActorComponent Object Reference")
    (`KismetArrayLibrary.Array_Add` (`self.NeonSidingArray`) _array_element)))