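; BP_SlidingDoor is a door that slides when a VRPawnLanguage enters or leaves its Collision component, or acts as an exit door.
; Begin and end overlap play separate Left and Right timelines, which drive the Door's relative Y location.
; If its Text3D label reads "Exit Game", either overlap event opens Map_LevelSelect instead, so the displayed text selects the behavior.
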(event `self.Collision.OnComponentBeginOverlap`
  (params (OverlappedComponent :type "PrimitiveComponent Object Reference") (OtherActor :type "Actor Object Reference") (OtherComp :type "PrimitiveComponent Object Reference") (OtherBodyIndex :type Integer) (bFromSweep :type Boolean) (SweepResult :type "HitResult Structure (by ref)"))
  (bind _door (`self.Door`))
  (bind (_relativelocation_x _relativelocation_y _relativelocation_z) (`KismetMathLibrary.BreakVector` (`SceneComponent.RelativeLocation` _door)))
  (cast `/Game/Language/Blueprints/VRPawnLanguage` OtherActor)
  (if (!= (`Text3DComponent.Text` (`self.Text3D`)) "Exit \nGame")
    (bind (_direction _left) (`Timeline|Left`)
      (:`Update`
        (`SceneComponent.K2_SetRelativeLocation` _door (`KismetMathLibrary.MakeVector` _relativelocation_x _left _relativelocation_z) false false)))
    (else
      (`GameplayStatics.OpenLevel` "Map_LevelSelect"))))

(event `self.Collision.OnComponentEndOverlap`
  (params (OverlappedComponent :type "PrimitiveComponent Object Reference") (OtherActor :type "Actor Object Reference") (OtherComp :type "PrimitiveComponent Object Reference") (OtherBodyIndex :type Integer))
  (bind _door (`self.Door`))
  (bind (_relativelocation_x _relativelocation_y _relativelocation_z) (`KismetMathLibrary.BreakVector` (`SceneComponent.RelativeLocation` _door)))
  (cast `/Game/Language/Blueprints/VRPawnLanguage` OtherActor)
  (if (!= (`Text3DComponent.Text` (`self.Text3D`)) "Exit \nGame")
    (bind (_direction _right) (`Timeline|Right`)
      (:`Update`
        (`SceneComponent.K2_SetRelativeLocation` _door (`KismetMathLibrary.MakeVector` _relativelocation_x _right _relativelocation_z) false false)))
    (else
      (`GameplayStatics.OpenLevel` "Map_LevelSelect"))))

(fn `UserConstructionScript`)