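; BP_Whiteboard is a drawable whiteboard that accumulates marker strokes in the RT_Whiteboard render target.
; On BeginPlay it clears the target to black and creates dynamic materials for the marker and the board mesh.
; DrawOnWhiteboard passes a 2D location to the marker's DrawLocation parameter and draws that material into the target.
; Despite its name, ChangeColor ignores its input and only clears the target to black.
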(event `self.ReceiveBeginPlay`
  (bind _returnvalue (`KismetMaterialLibrary.CreateDynamicMaterialInstance` "/Game/Drawing/Whiteboard/M_WhiteboardMarker.M_WhiteboardMarker"))
  (set `self.MI_WhiteBoardMarker` _returnvalue)
  (`KismetRenderingLibrary.ClearRenderTarget2D` "/Game/Drawing/Whiteboard/RT_Whiteboard.RT_Whiteboard")
  (`KismetMaterialLibrary.CreateDynamicMaterialInstance` "/Game/Drawing/Whiteboard/M_Whiteboard.M_Whiteboard")
  (bind _returnvalue_2 (`PrimitiveComponent.CreateDynamicMaterialInstance` (`self.Whiteboard`) 0 "/Game/Drawing/Whiteboard/M_Whiteboard.M_Whiteboard" "None"))
  (set `self.MI_WhiteboardMat` _returnvalue_2))

(event `DrawOnWhiteboard`
  (params (LocationToDraw :type "Vector2D Structure"))
  (bind _mi_whiteboardmarker (`self.MI_WhiteBoardMarker`))
  (`/Engine/EditorBlueprintResources/StandardMacros.IsValid` _mi_whiteboardmarker
    (:`Is Valid`
      (`MaterialInstanceDynamic.SetVectorParameterValue` _mi_whiteboardmarker "DrawLocation" (`KismetMathLibrary.Conv_VectorToLinearColor` (`KismetMathLibrary.Conv_Vector2DToVector` LocationToDraw)))
      (`KismetRenderingLibrary.DrawMaterialToRenderTarget` "/Game/Drawing/Whiteboard/RT_Whiteboard.RT_Whiteboard" _mi_whiteboardmarker))
    (:`Is Not Valid`
      (`KismetSystemLibrary.PrintString` "No Valid"))))

(event `ChangeColor`
  (params (vect :type "Vector Structure"))
  (`KismetRenderingLibrary.ClearRenderTarget2D` "/Game/Drawing/Whiteboard/RT_Whiteboard.RT_Whiteboard"))

(fn `UserConstructionScript`)