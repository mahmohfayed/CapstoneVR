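; BP_SplineStroke is a drawn stroke actor that builds a line out of spline mesh segments as a cursor moves.
; Each Update call adds a new SplineMeshComponent between the current and previous cursor locations, converted to actor-local space, then stores the current location.
; When the stored location is near zero, as on a first call, it only records the cursor location.
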(fn `CreateSplineMesh`
  (returns (NewSplineMesh :type "SplineMeshComponent Object Reference"))
  (bind _returnvalue (`AddComponent|NODE_AddSplineMeshComponent-0`))
  (`self.K2_AttachToComponent` _returnvalue "None" "SnapToTarget" "SnapToTarget" "SnapToTarget")
  (return _returnvalue))

(fn `Update`
  (params (CursorLocation :type "Vector Structure"))
  (locals (NewLocalVar_0 :type Boolean))
  (bind _returnvalue (`self.GetTransform`))
  (if (`KismetMathLibrary.Vector_IsNearlyZero` (`self.PreviousCursorLocation`))
    (set `self.PreviousCursorLocation` CursorLocation)
    (return)
    (else
      (bind _newsplinemesh (`self.CreateSplineMesh`))
      (`SplineMeshComponent.SetStartAndEnd` _newsplinemesh (`KismetMathLibrary.InverseTransformLocation` _returnvalue CursorLocation) (0.0 0.0 0.0) (`KismetMathLibrary.InverseTransformLocation` _returnvalue (`self.PreviousCursorLocation`)) (0.0 0.0 0.0) true)
      (set `self.PreviousCursorLocation` (`local.CursorLocation`)))))

(fn `UserConstructionScript`)