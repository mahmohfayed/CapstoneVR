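; Actor for one drawn stroke, which builds a visible trail from successive cursor locations passed to Update.
; Each update adds an instanced joint mesh at the cursor, converted to actor-local space.
; After the first point, it also adds an instanced segment at the current location, oriented by the movement vector and X-scaled to its length.
; A near-zero stored previous location marks the first point.
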(fn `GetNextJointTransform`
  (params (CurrentLocation :type "Vector Structure"))
  (returns (JointTransform :type "Transform Structure"))
  (locals (JointTrans :type "Transform Structure"))
  (bind _output_get (set `local.JointTrans` (`KismetMathLibrary.MakeTransform` (`KismetMathLibrary.InverseTransformLocation` (`self.GetTransform`) CurrentLocation))))
  (return _output_get))

(fn `GetNextSegmentLocation`
  (params (CurrentLocation :type "Vector Structure"))
  (returns (Location :type "Vector Structure"))
  (return (`KismetMathLibrary.InverseTransformLocation` (`self.GetTransform`) CurrentLocation)))

(fn `GetNextSegmentRotation`
  (params (CurrentLocation :type "Vector Structure"))
  (returns (Quat :type "Quat Structure"))
  (locals (Segment :type "Vector Structure") (SegmentNormal :type "Vector Structure") (NewLocalVar_0 :type "Quat Structure"))
  (bind _output_get (set `local.Segment` (- CurrentLocation (`self.PreviousCursorLocation`))))
  (return (`KismetMathLibrary.Conv_VectorToQuaternion` _output_get)))

(fn `GetNextSegmentScale`
  (params (CurrentLocation :type "Vector Structure"))
  (returns (Scale :type "Vector Structure"))
  (locals (Segment :type "Vector Structure"))
  (bind _output_get (set `local.Segment` (- CurrentLocation (`self.PreviousCursorLocation`))))
  (return (`KismetMathLibrary.MakeVector` (`KismetMathLibrary.VSize` _output_get) 1.0 1.0)))

(fn `GetNextSegmentTransform`
  (params (CurrentLocation :type "Vector Structure"))
  (returns (SegTransform :type "Transform Structure"))
  (locals (SegmentTransform :type "Transform Structure"))
  (bind _location (`self.GetNextSegmentLocation` CurrentLocation))
  (bind _quat (`self.GetNextSegmentRotation` CurrentLocation))
  (bind _scale (`self.GetNextSegmentScale` CurrentLocation))
  (bind _output_get (set `local.SegmentTransform` (`KismetMathLibrary.MakeTransform` _location (`KismetMathLibrary.Quat_Rotator` _quat) _scale)))
  (return _output_get))

(fn `Update`
  (params (CursorLocation :type "Vector Structure"))
  (locals (Spline :type "SplineMeshComponent Object Reference") (LocalCursorLocation :type "Vector Structure") (NewStrokeTransform :type "Transform Structure"))
  (bind _cursorlocation (`local.CursorLocation`))
  (bind _cursorlocation_2 (`local.CursorLocation`))
  (if (`KismetMathLibrary.Vector_IsNearlyZero` (`self.PreviousCursorLocation`))
    (set `self.PreviousCursorLocation` _cursorlocation_2)
    (bind _jointtransform (`self.GetNextJointTransform` _cursorlocation_2))
    (`InstancedStaticMeshComponent.AddInstance` (`self.InstSM_JointMeshes`) _jointtransform false)
    (return)
    (else
      (bind _segtransform (`self.GetNextSegmentTransform` _cursorlocation))
      (`InstancedStaticMeshComponent.AddInstance` (`self.InstSM_StrokeMeshes`) _segtransform false)
      (bind _jointtransform_2 (`self.GetNextJointTransform` _cursorlocation))
      (`InstancedStaticMeshComponent.AddInstance` (`self.InstSM_JointMeshes`) _jointtransform_2 false)
      (set `self.PreviousCursorLocation` (`local.CursorLocation`)))))

(fn `UserConstructionScript`)