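; Actor that hosts the grouped menus widget and exposes its level start choices to the rest of the game.
; On BeginPlay it casts the Widget component's widget to grouped_menus and binds to its start events for levels 0, 1 and 2.
; Each bound event rebroadcasts through the actor's own Start0, Start1 or Start2 dispatcher, so the level loading itself happens outside this Blueprint.
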(event `self.ReceiveBeginPlay`
  (bind _asgrouped_menus (cast `/Game/eVR_Content_Mahmoud/Blueprints/Widgets/grouped_menus` (`WidgetComponent.GetWidget` (`self.Widget`))))
  (add `/Game/eVR_Content_Mahmoud/Blueprints/Widgets/grouped_menus.start_lvl_0` _asgrouped_menus (delegate `start_lvl_0_Event_0`))
  (add `/Game/eVR_Content_Mahmoud/Blueprints/Widgets/grouped_menus.start_lvl_1` _asgrouped_menus (delegate `start_lvl_1_Event_0`))
  (add `/Game/eVR_Content_Mahmoud/Blueprints/Widgets/grouped_menus.start_lvl_2` _asgrouped_menus (delegate `start_lvl_2_Event_0`)))

(event `start_lvl_0_Event_0`
  (`self.start_0`))

(event `start_lvl_1_Event_0`
  (`self.start_1`))

(event `start_lvl_2_Event_0`
  (`self.start_2`))

(fn `UserConstructionScript`)