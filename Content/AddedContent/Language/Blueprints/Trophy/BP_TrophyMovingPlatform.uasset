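; Trophy moving platform actor that shuttles its Cube along a timeline-driven path.
; From BeginPlay it waits through a fixed delay, then plays or reverses the timeline based on the Loop flag, with JustCreated forcing a forward first run when Loop is set.
; Timeline updates set the Cube's relative location without sweep, and each finish flips Loop and re-enters the delay.
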(event `self.ReceiveBeginPlay`
  (`KismetSystemLibrary.Delay` 5.0 :!label _label)
  (if (`self.Loop`)
    (if (`self.JustCreated`)
      (set `self.JustCreated` false)
      (bind (_direction _newtrack_0) (`Timeline|Timeline_0` :!label _label_2)
        (:`Update`
          (`SceneComponent.K2_SetRelativeLocation` (`self.Cube`) _newtrack_0 false false))
        (:`Finished`
          (if (`self.Loop`)
            (set `self.Loop` false)
            (goto _label)
            (else
              (set `self.Loop` true)
              (goto _label)))))
      (else
        (goto _label_2 :!via `Reverse`)))
    (else
      (goto _label_2))))

(fn `UserConstructionScript`)