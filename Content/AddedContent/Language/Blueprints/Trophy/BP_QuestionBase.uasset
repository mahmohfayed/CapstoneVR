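; Base actor for a VR trophy quiz station showing one question with three answer rings.
; CreateBases fills widget components with the supplied texts, stores the correct answer and finds the BP_TrophyCountBoard.
; The hidden station appears when the BP_VRPawn overlaps its collision.
; The first ring touched locks all three, turning green and adding a trophy to the board if correct, otherwise red, with matching sound.
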(event `self.ReceiveBeginPlay`
  (`SceneComponent.SetVisibility` (`self.Root`) false true))

(event `CreateBases`
  (params (Question_text :type Text) (answer_1 :type Text) (answer_2 :type Text) (answer_3 :type Text) (correct_answer :type Integer))
  ;[1 1 1] Prepare Trophy Base
  (`|ExecutionSequence`
    (:`then_0`
      (bind _returnvalue (`|CreateWidget` "/Game/AddedContent/Language/Blueprints/Trophy/WBP_Question.WBP_Question_C" null Question_text))
      (`WidgetComponent.SetWidget` (`self.Question`) _returnvalue)
      (bind _returnvalue_2 (`|CreateWidget` "/Game/AddedContent/Language/Blueprints/Trophy/WBP_Question.WBP_Question_C" null answer_1))
      (`WidgetComponent.SetWidget` (`self.Answer1`) _returnvalue_2)
      (bind _returnvalue_3 (`|CreateWidget` "/Game/AddedContent/Language/Blueprints/Trophy/WBP_Question.WBP_Question_C" null answer_2))
      (`WidgetComponent.SetWidget` (`self.Answer2`) _returnvalue_3)
      (bind _returnvalue_4 (`|CreateWidget` "/Game/AddedContent/Language/Blueprints/Trophy/WBP_Question.WBP_Question_C" null answer_3))
      (`WidgetComponent.SetWidget` (`self.Answer3`) _returnvalue_4)
      (set `self.correct_answer` correct_answer)
      (bind _returnvalue_5 (`GameplayStatics.GetActorOfClass` "/Game/AddedContent/Language/Blueprints/Points/BP_TrophyCountBoard.BP_TrophyCountBoard_C"))
      (set `self.Point Board` _returnvalue_5))
    (:`then_1`
      (`SceneComponent.SetVisibility` (`self.Answer1`) false false)
      (`SceneComponent.SetVisibility` (`self.Answer2`) false false)
      (`SceneComponent.SetVisibility` (`self.Answer3`) false false)
      (`SceneComponent.SetVisibility` (`self.Question`) false false)
      (`SceneComponent.SetVisibility` (`self.AnswerRing1`) false false)
      (`SceneComponent.SetVisibility` (`self.AnswerRing2`) false false)
      (`SceneComponent.SetVisibility` (`self.AnswerRing3`) false false)
      (`PrimitiveComponent.SetMaterial` (`self.Cone`) 0 "/Game/AddedContent/Language/Materials/M_Emissive_White.M_Emissive_White"))))

(event `self.Collision.OnComponentBeginOverlap`
  (params (OverlappedComponent :type "PrimitiveComponent Object Reference") (OtherActor :type "Actor Object Reference") (OtherComp :type "PrimitiveComponent Object Reference") (OtherBodyIndex :type Integer) (bFromSweep :type Boolean) (SweepResult :type "HitResult Structure (by ref)"))
  ;[1 0.9704 0.1156] Set Visible when Approaching
  (cast `/Game/Fundamental/Blueprints/Pawn/BP_VRPawn` OtherActor)
  (`SceneComponent.SetVisibility` (`self.Root`) true true)
  (`PrimitiveComponent.SetMaterial` (`self.Cone`) 0 "/Game/AddedContent/Language/Materials/M_Tech_Hex_Tile_Pulse.M_Tech_Hex_Tile_Pulse")
  (set `PrimitiveComponent.bGenerateOverlapEvents` false (`self.Collision`)))

(event `self.AnswerRing1.OnComponentBeginOverlap`
  (params (OverlappedComponent :type "PrimitiveComponent Object Reference") (OtherActor :type "Actor Object Reference") (OtherComp :type "PrimitiveComponent Object Reference") (OtherBodyIndex :type Integer) (bFromSweep :type Boolean) (SweepResult :type "HitResult Structure (by ref)"))
  ;[0.04342 1 0.1768] Check Answer
  (cast `/Game/Fundamental/Blueprints/Pawn/BP_VRPawn` OtherActor)
  (if (== (`self.correct_answer`) 1)
    (`self.SetGreen` OverlappedComponent)
    (else
      (`self.SetRed` OverlappedComponent))))

(event `self.AnswerRing2.OnComponentBeginOverlap`
  (params (OverlappedComponent :type "PrimitiveComponent Object Reference") (OtherActor :type "Actor Object Reference") (OtherComp :type "PrimitiveComponent Object Reference") (OtherBodyIndex :type Integer) (bFromSweep :type Boolean) (SweepResult :type "HitResult Structure (by ref)"))
  ;[0.04342 1 0.1768] Check Answer
  (cast `/Game/Fundamental/Blueprints/Pawn/BP_VRPawn` OtherActor)
  (if (== (`self.correct_answer`) 2)
    (`self.SetGreen` OverlappedComponent)
    (else
      (`self.SetRed` OverlappedComponent))))

(event `self.AnswerRing3.OnComponentBeginOverlap`
  (params (OverlappedComponent :type "PrimitiveComponent Object Reference") (OtherActor :type "Actor Object Reference") (OtherComp :type "PrimitiveComponent Object Reference") (OtherBodyIndex :type Integer) (bFromSweep :type Boolean) (SweepResult :type "HitResult Structure (by ref)"))
  ;[0.04342 1 0.1768] Check Answer
  (cast `/Game/Fundamental/Blueprints/Pawn/BP_VRPawn` OtherActor)
  (if (== (`self.correct_answer`) 3)
    (`self.SetGreen` OverlappedComponent)
    (else
      (`self.SetRed` OverlappedComponent))))

(fn `DisableCollisions`
  (set `PrimitiveComponent.bGenerateOverlapEvents` false (`self.AnswerRing1`))
  (set `PrimitiveComponent.bGenerateOverlapEvents` false (`self.AnswerRing2`))
  (set `PrimitiveComponent.bGenerateOverlapEvents` false (`self.AnswerRing3`)))

(fn `SetGreen`
  (params (Ring :type "PrimitiveComponent Object Reference"))
  (`PrimitiveComponent.SetMaterial` Ring 0 "/Game/AddedContent/Language/Materials/M_Emissive_Green.M_Emissive_Green")
  (`self.DisableCollisions`)
  (`SceneComponent.SetVisibility` (`self.Question`) false false)
  (`/Game/AddedContent/Language/Blueprints/Points/BP_TrophyCountBoard.Add_Trophy` (`self.Point Board`))
  (`GameplayStatics.PlaySound2D` "/Game/AddedContent/Language/Sounds/light-pop.light-pop" 1.0 1.0 0.0 null null))

(fn `SetRed`
  (params (Ring :type "PrimitiveComponent Object Reference"))
  (`PrimitiveComponent.SetMaterial` Ring 0 "/Game/AddedContent/Language/Materials/M_Emissive_Red.M_Emissive_Red")
  (`self.DisableCollisions`)
  (`GameplayStatics.PlaySound2D` "/Game/AddedContent/Language/Sounds/wrong-buzzer.wrong-buzzer" 1.0 1.0 0.0 null null))

(fn `UserConstructionScript`)