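; BP_PuzzleBoard runs a slot-and-piece puzzle, registering its child slots and gathering all puzzle pieces at BeginPlay.
; ReleasePieces moves four random pieces to preset transforms, then after a delay messages the Language level Blueprint to restart.
; CheckAllCorrect plays a sound when every slot is correct and requests a restart with a new puzzle.
; BPI_Puzzle carries both requests, targeting actors by name; ClearPuzzleBoard destroys slotted pieces.
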(event `self.ReceiveBeginPlay`
  ;[1 1 1] Set Up Slot Array
  (for _array_element (`SceneComponent.GetChildrenComponents` (`self.DefaultSceneRoot`) false)
    (bind _aschild_actor_component (cast `ChildActorComponent` _array_element))
    (bind _asbp_puzzle_slot (cast `/Game/AddedContent/Language/Blueprints/Puzzles/Puzzle/BP_PuzzleSlot` (`ChildActorComponent.ChildActor` _aschild_actor_component)))
    (`KismetArrayLibrary.Array_Add` (`self.SlotArray`) _asbp_puzzle_slot)
    (set `/Game/AddedContent/Language/Blueprints/Puzzles/Puzzle/BP_PuzzleSlot.PuzzleBoardRef` self _asbp_puzzle_slot))
  (bind _outactors (`GameplayStatics.GetAllActorsOfClass` "/Game/AddedContent/Language/Blueprints/Puzzles/Puzzle/BP_PuzzlePiece.BP_PuzzlePiece_C"))
  (set `self.PuzzlePieceArray` _outactors))

(event `ReleasePieces`
  (bind _puzzlepiecearray (`self.PuzzlePieceArray`))
  (bind _currentpuzzlepiece (`self.CurrentPuzzlePiece`))
  (bind (_outitem _outindex) (`KismetArrayLibrary.Array_Random` _puzzlepiecearray))
  ;[0.4033 0.5595 1] Release pieces in groups of 4
  (`/Engine/EditorBlueprintResources/StandardMacros.DoOnce` false :!label _label
    (:`Completed`
      (for _index (range 4)
        (bind _output_get (set `self.CurrentPuzzlePiece` _outitem :!label _label_2))
        (set `self.CurrentPieceInt` _outindex)
        (`/Engine/EditorBlueprintResources/StandardMacros.IsValid` _output_get
          (:`Is Valid`
            (`self.K2_SetActorTransform` _currentpuzzlepiece (`|GetArrayItem` (`self.Transforms`) _index) false false)
            (`KismetArrayLibrary.Array_RemoveItem` _puzzlepiecearray _currentpuzzlepiece))
          (:`Is Not Valid`
            (goto _label_2))))
      (`KismetSystemLibrary.Delay` 10.0)
      (`|ExecutionSequence`
        (:`then_0`
          ;[1 0.1349 0.1249] Contact level blueprint to restart level
          (bind _outactors (`GameplayStatics.GetAllActorsWithInterface` "/Game/AddedContent/Language/Blueprints/Puzzles/Puzzle/BPI_Puzzle.BPI_Puzzle_C"))
          (for _array_element _outactors
            (if (`KismetStringLibrary.Contains` (`KismetSystemLibrary.GetObjectName` _array_element) "Language")
              (`/Engine/EditorBlueprintResources/StandardMacros.DoOnce` false :!label _label_3
                (:`Completed`
                  (message `/Game/AddedContent/Language/Blueprints/Puzzles/Puzzle/BPI_Puzzle.BPI Restart Level` _array_element)))))
          (goto _label_3 :!via `Reset`))
        (:`then_1`
          (goto _label :!via `Reset`))))))

(event `CheckAllCorrect`
  ;[1 0.6325 0.5424] Check if Slots are Filled and Correct
  (for _array_element (`self.SlotArray`)
    (if (`/Game/AddedContent/Language/Blueprints/Puzzles/Puzzle/BP_PuzzleSlot.Correct` _array_element)
      (set `self.AllCorrect` true)
      (else
        (set `self.AllCorrect` false)
        (break))))
  (if (`self.AllCorrect`)
    (`GameplayStatics.PlaySound2D` "/Game/AddedContent/Interface_And_Item_Sounds/WAV/Coins_15.Coins_15" 1.0 1.0 0.0 null null)
    (set `self.Completed` true)
    ;[1 0.1349 0.1249] Contact level blueprint to restart level with new puzzle
    (bind _outactors (`GameplayStatics.GetAllActorsWithInterface` "/Game/AddedContent/Language/Blueprints/Puzzles/Puzzle/BPI_Puzzle.BPI_Puzzle_C"))
    (for _array_element_2 _outactors
      (if (`KismetStringLibrary.Contains` (`KismetSystemLibrary.GetObjectName` _array_element_2) "Language")
        (`/Engine/EditorBlueprintResources/StandardMacros.DoOnce` false :!label _label_4
          (:`Completed`
            (message `/Game/AddedContent/Language/Blueprints/Puzzles/Puzzle/BPI_Puzzle.BPIRestartLevelWPuzzle` _array_element_2)))))
    (goto _label_4 :!via `Reset`)))

(event `ClearPuzzleBoard`
  ;[1 0.5895 0.8338] Remove all Puzzle Pieces
  (for _array_element (`self.SlotArray`)
    (`self.K2_DestroyActor` (`/Game/AddedContent/Language/Blueprints/Puzzles/Puzzle/BP_PuzzleSlot.CurrentPiece` _array_element))))

(fn `UserConstructionScript`)