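; Sentence translation puzzle display that checks whether every word slot is filled correctly and, on success, tells its puzzle board to release pieces.
; CreateTranslateDisplay shows the original sentence in a widget and spawns a row of block slots, each assigned a word to match.
; Overlapping the box collision, moved to a fixed world position at BeginPlay, checks all slots and plays success or failure audio.
; A DoOnce limits piece release until the overlap ends; DeleteBlockSlots destroys the slots.
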(event `self.ReceiveBeginPlay`
  (`SceneComponent.K2_SetWorldLocation` (`self.BoxCollision`) (465.91864 -682.0 32.755577) false false))

(event `CreateTranslateDisplay`
  (params (`Puzzle Board` :type "/Game/AddedContent/Language/Blueprints/Puzzles/Puzzle/BP_PuzzleBoard Object Reference") (CheckSentences :type "TriggerBox Object Reference"))
  (bind _blocktransform (`self.BlockTransform`))
  (set `self.PuzzleBoardRef` `Puzzle Board`)
  (`|ExecutionSequence`
    (:`then_0`
      ;[1 0.8394 0.5265] Set SentenceWidget
      (bind _returnvalue (`|CreateWidget` "/Game/AddedContent/Language/Blueprints/Puzzles/Sentences/WBP_Sentences.WBP_Sentences_C" null (`self.OriginalSentence`)))
      (`WidgetComponent.SetWidget` (`self.SentenceWidget`) _returnvalue))
    (:`then_1`
      ;[0.5521 1 1] Create Block Slots
      (for _index (range (`KismetArrayLibrary.Array_Length` (`self.WordArray`)))
        (bind _output_get (set `self.Tranforms` (`KismetMathLibrary.MakeTransform` (`KismetMathLibrary.MakeVector` (+ (.x (.location _blocktransform)) (* _index 60)) (.y (.location _blocktransform)) (.z (.location _blocktransform))) (.rotation _blocktransform) (.scale _blocktransform))))
        (bind _returnvalue_2 (`|SpawnActorFromClass` "/Game/AddedContent/Language/Blueprints/Puzzles/Sentences/BP_SentenceBlockSlot.BP_SentenceBlockSlot_C" _output_get "Undefined" "OverrideRootScale" null self 0 null null))
        (`KismetArrayLibrary.Array_Add` (`self.BlockSlots`) _returnvalue_2)
        ;[0.6461 0.7205 1] Set Word to Match
        (bind _output_get_2 (set `/Game/AddedContent/Language/Blueprints/Puzzles/Sentences/BP_SentenceBlockSlot.WordToMatch` (`KismetTextLibrary.Conv_StringToText` (`|GetArrayItem` (`self.WordArray`) _index)) _returnvalue_2))
        (`TextRenderComponent.K2_SetText` (`/Game/AddedContent/Language/Blueprints/Puzzles/Sentences/BP_SentenceBlockSlot.WordMatchText` _returnvalue_2) _output_get_2) ; for editing purposes only
      ))))

(event `self.BoxCollision.OnComponentBeginOverlap`
  (params (OverlappedComponent :type "PrimitiveComponent Object Reference") (OtherActor :type "Actor Object Reference") (OtherComp :type "PrimitiveComponent Object Reference") (OtherBodyIndex :type Integer) (bFromSweep :type Boolean) (SweepResult :type "HitResult Structure (by ref)"))
  ;[1 0.9928 0.6588] Check if all slots are correct
  (for _array_element (`self.BlockSlots`)
    (bind _bcorrect (`/Game/AddedContent/Language/Blueprints/Puzzles/Sentences/BP_SentenceBlockSlot.Return Block Correct` _array_element))
    (if _bcorrect
      (set `self.AllCorrect` true)
      (else
        (set `self.AllCorrect` false)
        (break))))
  (if (`self.AllCorrect`)
    (`GameplayStatics.PlaySound2D` "/Game/AddedContent/Interface_And_Item_Sounds/WAV/Coins_15.Coins_15" 1.0 1.0 0.0 null null)
    (`/Engine/EditorBlueprintResources/StandardMacros.DoOnce` false :!label _label
      (:`Completed`
        (`/Game/AddedContent/Language/Blueprints/Puzzles/Puzzle/BP_PuzzleBoard.ReleasePieces` (`self.PuzzleBoardRef`))))
    (else
      (`GameplayStatics.PlaySound2D` "/Game/AddedContent/Language/Sounds/wrong-buzzer.wrong-buzzer" 1.0 1.0 0.0 null null))))

(event `self.BoxCollision.OnComponentEndOverlap`
  (params (OverlappedComponent :type "PrimitiveComponent Object Reference") (OtherActor :type "Actor Object Reference") (OtherComp :type "PrimitiveComponent Object Reference") (OtherBodyIndex :type Integer))
  ;[1 0.9928 0.6588] Check if all slots are correct
  (goto _label :!via `Reset`))

(event `DeleteBlockSlots`
  ;[0.7413 0.8271 1] Delete Block Slots
  (bind (_arrayindex _arrayelement) (`/Engine/EditorBlueprintResources/StandardMacros.ReverseForEachLoop` (`self.BlockSlots`))
    (:`LoopBody`
      (`self.K2_DestroyActor` _arrayelement))))

(fn `UserConstructionScript`)