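; BP_VocabPointsBoard is an actor that serves as a points board, apparently for a vocabulary game.
; On BeginPlay it creates a WBP_VocabPoints widget, passing in the initial PointsInt value, and assigns it to its Points widget component.
; Add_Point and SubtractPoints change the count by one and play a pop or buzzer sound, with no explicit widget refresh.
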(event `self.ReceiveBeginPlay`
  (bind _returnvalue (`|CreateWidget` "/Game/AddedContent/Language/Blueprints/Points/WBP_VocabPoints.WBP_VocabPoints_C" null (`self.Points Int`)))
  (`WidgetComponent.SetWidget` (`self.Points`) _returnvalue))

(event `Add_Point`
  (set `self.Points Int` (+ (`self.Points Int`) 1))
  (`GameplayStatics.PlaySound2D` "/Game/AddedContent/Language/Sounds/light-pop.light-pop" 1.0 1.0 0.0 null null))

(event `SubtractPoints`
  (set `self.Points Int` (- (`self.Points Int`) 1))
  (`GameplayStatics.PlaySound2D` "/Game/AddedContent/Language/Sounds/wrong-buzzer.wrong-buzzer" 1.0 1.0 0.0 null null))

(fn `UserConstructionScript`)