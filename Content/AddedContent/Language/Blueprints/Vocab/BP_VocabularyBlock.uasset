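; Grabbable vocabulary word block for a language game, with neon edging that turns green or red for correct or wrong answers.
; On BeginPlay it creates one text widget from BlockText, assigns it to six word components and sets a lifespan.
; Grab and Drop toggle physics and attachment.
; CreateExtraHits binds a hit handler that, once only, turns the neon red and subtracts points on contact with a vocab target.
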(event `CreateExtraHits`
  (params (PointsBoard :type "/Game/AddedContent/Language/Blueprints/Points/BP_VocabPointsBoard Object Reference"))
  ;[1 0.2486 0.7981] Hit Event - Subtract
  (add `self.OnActorHit` (delegate `ExtraBlockHits`)))

(event `ExtraBlockHits` :!signature `self.OnActorHit`
  (params (SelfActor :type "Actor Object Reference") (OtherActor :type "Actor Object Reference") (NormalImpulse :type "Vector Structure") (Hit :type "HitResult Structure (by ref)"))
  ;[1 0.2486 0.7981] Hit Event - Subtract
  (cast `/Game/AddedContent/Language/Blueprints/Vocab/BP_VocabTarget` OtherActor)
  (`/Engine/EditorBlueprintResources/StandardMacros.DoOnce` false
    (:`Completed`
      (`self.ChangeWrong`)
      (`/Game/AddedContent/Language/Blueprints/Points/BP_VocabPointsBoard.SubtractPoints` (stale `CreateExtraHits` PointsBoard))
      (`KismetSystemLibrary.Delay` 1.5))))

(event `self.ReceiveBeginPlay`
  ;[0.461 0.5606 1] Create Word Widgets (Surface)
  (bind _returnvalue (`|CreateWidget` "/Game/AddedContent/Language/Blueprints/Vocab/WBP_VocabText.WBP_VocabText_C" null (`self.Block Text`)))
  (`WidgetComponent.SetWidget` (`self.Word1`) _returnvalue)
  (`WidgetComponent.SetWidget` (`self.Word2`) _returnvalue)
  (`WidgetComponent.SetWidget` (`self.Word3`) _returnvalue)
  (`WidgetComponent.SetWidget` (`self.Word4`) _returnvalue)
  (`WidgetComponent.SetWidget` (`self.Word5`) _returnvalue)
  (`WidgetComponent.SetWidget` (`self.Word6`) _returnvalue)
  (`self.SetLifeSpan` (`self.Lifespan`)))

(event `/Game/Fundamental/Blueprints/Interface/BPI_GrabbaleActor.Grab`
  (params (AttachTo :type "SceneComponent Object Reference"))
  ;[1 1 1] Set Grabbable
  (`PrimitiveComponent.SetSimulatePhysics` (`self.Cube`) false)
  (`SceneComponent.K2_AttachToComponent` (`self.RootComponent`) AttachTo "None" "KeepWorld" "KeepWorld" "KeepWorld" false))

(event `ChangeCorrect`
  ;[0.02494 1 0.1983] Correct Neon
  (for _array_element (`self.NeonSidingArray`)
    (bind _asbp_neon_siding (cast `/Game/AddedContent/Language/Blueprints/BP_NeonSiding` (`ChildActorComponent.ChildActor` _array_element)))
    (`/Game/AddedContent/Language/Blueprints/BP_NeonSiding.Change Material` _asbp_neon_siding "/Game/AddedContent/Language/Materials/MI_Emissive_Green.MI_Emissive_Green")))

(event `ChangeWrong`
  ;[1 0.09279 0.1326] Wrong Neon
  (for _array_element (`self.NeonSidingArray`)
    (bind _asbp_neon_siding (cast `/Game/AddedContent/Language/Blueprints/BP_NeonSiding` (`ChildActorComponent.ChildActor` _array_element)))
    (`/Game/AddedContent/Language/Blueprints/BP_NeonSiding.Change Material` _asbp_neon_siding "/Game/AddedContent/Language/Materials/MI_Emissive_Red.MI_Emissive_Red")))

(event `/Game/Fundamental/Blueprints/Interface/BPI_GrabbaleActor.Drop`
  ;[1 1 1] Set Grabbable
  (`PrimitiveComponent.SetSimulatePhysics` (`self.Cube`) true)
  (`self.K2_DetachFromActor` "KeepWorld" "KeepWorld" "KeepWorld"))

(fn `UserConstructionScript`
  (for _array_element (`|MakeArray` (`self.NeonSiding`) (`self.NeonSiding1`) (`self.NeonSiding2`) (`self.NeonSiding3`) (`self.NeonSiding4`) (`self.NeonSiding5`) (`self.NeonSiding6`) (`self.NeonSiding7`))
    (`KismetArrayLibrary.Array_Add` (`self.NeonSidingArray`) _array_element)))